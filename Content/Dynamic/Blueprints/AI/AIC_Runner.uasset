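; AIC_Runner is an AI controller that drives a possessed BP_Runner by simulating its left and right power inputs.
; On possession it caches the runner, and from BeginPlay it starts a one-shot timer with a random delay between minimum and maximum input values.
; A FlipFlop alternates left and right power calls on the runner, rescheduling the timer after each.
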(event `self.ReceiveBeginPlay`
  (`self.SimluateInputWithDelay`))

(event `self.ReceivePossess`
  (params (PossessedPawn :type "Pawn Object Reference"))
  (bind _asbp_runner (cast `/Game/Dynamic/Blueprints/BP_Runner` PossessedPawn))
  (set `self.OwningRunner` _asbp_runner))

(event `SimulateInput`
  (`/Engine/EditorBlueprintResources/StandardMacros.FlipFlop`
    (:`A`
      (`/Game/Dynamic/Blueprints/BP_Runner.SimulatePowerLeft` (`self.OwningRunner`))
      (`self.SimluateInputWithDelay`))
    (:`B`
      (`/Game/Dynamic/Blueprints/BP_Runner.SimulatePowerRight` (`self.OwningRunner`))
      (`self.SimluateInputWithDelay`))))

(fn `SimluateInputWithDelay`
  (`KismetSystemLibrary.K2_SetTimerDelegate` (`|CreateDelegate` :!event `SimulateInput`) (`KismetMathLibrary.RandomFloatInRange` (`self.MinInputDelay`) (`self.MaxInputDelay`))))

(fn `UserConstructionScript`)